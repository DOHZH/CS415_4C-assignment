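; BP_AOE is an area-of-effect actor that applies damage to the player while they stand inside its sphere.
; Sphere overlaps toggle its damage flag and the player's InAoe flag, using the ThirdPersonCharacter found at BeginPlay.
; While active, Tick applies a small negative damage value every frame, making the rate framerate-dependent.
; Destruction clears both flags.
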(event OnComponentBeginOverlap(Sphere)
  (params (OverlappedComponent :type Primitive%20Component%20Object%20Reference) (OtherActor :type Actor%20Object%20Reference) (OtherComp :type Primitive%20Component%20Object%20Reference) (OtherBodyIndex :type Integer) (bFromSweep :type Boolean) (SweepResult :type Hit%20Result%20Structure%20%28by%20ref%29))
  (if (== OtherActor (Variables|Default|GetPlayer))
    (Variables|Default|SetStartAoeDamage true)
    (Variables|/Game/ThirdPersonCPP/Blueprints/ThirdPersonCharacter.ThirdPersonCharacter_C|SetInAoe (Variables|Default|GetPlayer) true)))

(event OnComponentEndOverlap(Sphere)
  (params (OverlappedComponent :type Primitive%20Component%20Object%20Reference) (OtherActor :type Actor%20Object%20Reference) (OtherComp :type Primitive%20Component%20Object%20Reference) (OtherBodyIndex :type Integer))
  (if (== OtherActor (Variables|Default|GetPlayer))
    (Variables|Default|SetStartAoeDamage false)
    (Variables|/Game/ThirdPersonCPP/Blueprints/ThirdPersonCharacter.ThirdPersonCharacter_C|SetInAoe (Variables|Default|GetPlayer) false)))

(event EventBeginPlay
  (bind _returnvalue (Actor|GetActorOfClass "/Game/ThirdPersonCPP/Blueprints/ThirdPersonCharacter.ThirdPersonCharacter_C"))
  (Variables|Default|SetPlayer _returnvalue))

(event EventTick
  (params (DeltaSeconds :type Float%20%28single-precision%29))
  (if (Variables|Default|GetStartAoeDamage)
    (Game|Damage|ApplyDamage (Variables|Default|GetPlayer) -0.5 0 0)))

(event EventDestroyed
  (Variables|Default|SetStartAoeDamage false)
  (Variables|/Game/ThirdPersonCPP/Blueprints/ThirdPersonCharacter.ThirdPersonCharacter_C|SetInAoe (Variables|Default|GetPlayer) false))

(fn ConstructionScript)