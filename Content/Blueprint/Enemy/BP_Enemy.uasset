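; Enemy whose defeat wins the game, with a melee component snapped to its mesh's axe socket during construction.
; It creates a viewport health bar on BeginPlay and updates it as AnyDamage lowers HP.
; Heavy non-lethal hits play an impact montage.
; The death check subtracts Damage again from the reduced HP, then plays a slowed death montage, destroys the actor, shows the Success widget and pauses the game.
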(event EventBeginPlay
  (bind _returnvalue (UserInterface|CreateWidget "/Game/UI/HealthBar.HealthBar_C"))
  (bind _output_get (Variables|Default|Sethealthbar _returnvalue))
  (UserInterface|Viewport|AddtoViewport _output_get 0))

(event Collision|EventActorBeginOverlap
  (params (OtherActor :type Actor%20Object%20Reference)))

(event EventTick
  (params (DeltaSeconds :type Float%20%28single-precision%29)))

(event Game|Damage|EventAnyDamage
  (params (Damage :type Float%20%28single-precision%29) (DamageType :type Damage%20Type%20Object%20Reference) (InstigatedBy :type Controller%20Object%20Reference) (DamageCauser :type Actor%20Object%20Reference))
  (bind _mesh (Variables|Character|GetMesh))
  (bind _returnvalue (Components|SkeletalMesh|GetAnimInstance _mesh))
  (bind _output_get (Variables|Default|SetHP (- (Variables|Default|GetHP) Damage)))
  (Progress|SetPercent (Variables|/Game/UI/HealthBar.HealthBar_C|GetProgressBar_33 (Variables|Default|Gethealthbar)) (Math|Float|SelectFloat 0.0 (/ _output_get 2e+02) (<= (- (Variables|Default|GetHP) Damage) 0.0)))
  (if (<= (- (Variables|Default|GetHP) Damage) 0.0)
    (bind _returnvalue_2 (Animation|Montage|MontagePlay _returnvalue "/Game/Mannequin/ActionAnima/Montage/Death.Death" 0.5 "MontageLength" 0.0 true))
    (Utilities|FlowControl|Delay (* _returnvalue_2 1.8))
    (Actor|DestroyActor)
    (bind _returnvalue_3 (UserInterface|CreateWidget "/Game/UI/Success.Success_C"))
    (UserInterface|Viewport|AddtoViewport _returnvalue_3 0)
    (Game|SetGamePaused true)
    (elif (> Damage 3e+01)
      (Animation|Montage|MontagePlay _returnvalue "/Game/Mannequin/ActionAnima/Montage/IsImpact.IsImpact" 1.0 "MontageLength" 0.0 true))))

(fn ConstructionScript
  (Transformation|AttachComponentToComponent (Variables|Default|GetMelee) (Variables|Character|GetMesh) "Axe_Attack" "SnapToTarget" "SnapToTarget" "SnapToTarget" true))