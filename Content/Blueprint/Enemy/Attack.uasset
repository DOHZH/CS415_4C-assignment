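; Behavior tree task that makes a BP_Enemy turn toward the player's ThirdPersonCharacter and attack.
; If HP is above zero, it plays either Enemy_Attack_1 or the BPA_Aoe montage at even odds.
; HP is read from the first BP_Enemy in the world, not the controlled pawn.
; The task finishes as failed when the montage completes or is interrupted, and never finishes when HP is depleted.
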(event EventReceiveExecuteAI
  (params (OwnerController :type AI%20Controller%20Object%20Reference) (ControlledPawn :type Pawn%20Object%20Reference))
  (bind _asbp_enemy (Utilities|Casting|CastToBP_Enemy ControlledPawn))
  (bind _returnvalue (Actor|GetActorOfClass "/Game/ThirdPersonCPP/Blueprints/ThirdPersonCharacter.ThirdPersonCharacter_C"))
  (Transformation|SetActorRotation _asbp_enemy (Math|Rotator|FindLookatRotation (Transformation|GetWorldLocation (Variables|/Script/Engine.Character|GetMesh _asbp_enemy)) (Transformation|GetWorldLocation (Variables|/Script/Engine.Character|GetMesh _returnvalue))))
  (bind _returnvalue_2 (Actor|GetActorOfClass "/Game/Blueprint/Enemy/BP_Enemy.BP_Enemy_C"))
  (if (not (<= (Variables|/Game/Blueprint/Enemy/BP_Enemy.BP_Enemy_C|GetHP _returnvalue_2) 0.0))
    (if (Math|Random|RandomBoolwithWeight 0.5)
      (Animation|Montage|PlayMontage (Variables|/Script/Engine.Character|GetMesh _asbp_enemy) "/Game/Blueprint/Enemy/Enemy_Attack_1.Enemy_Attack_1"
        (:OnCompleted
          _)
        (:OnInterrupted
          _))
      (AI|BehaviorTree|FinishExecute false)
      (else
        (Animation|Montage|PlayMontage (Variables|/Script/Engine.Character|GetMesh _asbp_enemy) "/Game/Blueprint/Enemy/BPA_Aoe.BPA_Aoe"
          (:OnCompleted
            _)
          (:OnInterrupted
            _))
        (AI|BehaviorTree|FinishExecute false)))))