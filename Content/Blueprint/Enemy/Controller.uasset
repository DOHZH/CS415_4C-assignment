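; Enemy AI controller that starts the BT_Enemy behavior tree and reports sightings of the player to it.
; On BeginPlay it runs the tree and caches the player character as a ThirdPersonCharacter.
; When PawnSensing sees that pawn, it writes it to the PlayerActor blackboard key.
; Nothing in this graph clears the key afterward.
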(event OnSeePawn(PawnSensing)
  (params (Pawn :type Pawn%20Object%20Reference))
  (bind _player (Variables|Default|GetPlayer))
  (if (== Pawn _player)
    (AI|Components|Blackboard|SetValueasObject (Variables|Default|GetBlackboard) (Variables|Default|GetPlayerActor) _player)))

(event EventBeginPlay
  (AI|RunBehaviorTree "/Game/Blueprint/Enemy/BT_Enemy.BT_Enemy")
  (bind _asthird_person_character (Utilities|Casting|CastToThirdPersonCharacter (Game|GetPlayerCharacter 0)))
  (Variables|Default|SetPlayer _asthird_person_character))

(event EventTick
  (params (DeltaSeconds :type Float%20%28single-precision%29)))

(fn ConstructionScript)