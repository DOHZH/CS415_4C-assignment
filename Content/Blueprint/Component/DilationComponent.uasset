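; DilationComponent is an actor component that slows its owning actor's time when its dilation flag is set.
; BeginPlay caches the owner once, guarded by an init flag.
; Every Tick it writes the owner's CustomTimeDilation, either slowed or normal speed, based on IsDilating, which nothing in this graph sets.
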(event EventBeginPlay
  (if (not (Variables|Default|GetIsInitied))
    (Variables|Default|SetIsInitied true)
    (Variables|Default|SetOwner (Components|GetOwner))))

(event EventTick
  (params (DeltaSeconds :type Float%20%28single-precision%29))
  (if (Variables|Default|GetIsInitied)
    (if (Variables|Default|GetIsDilating)
      (Variables|/Script/Engine.Actor|SetCustomTimeDilation (Variables|Default|GetOwner) 0.1)
      (else
        (Variables|/Script/Engine.Actor|SetCustomTimeDilation (Variables|Default|GetOwner) 1.0)))))