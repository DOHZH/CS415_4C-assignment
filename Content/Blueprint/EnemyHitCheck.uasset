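; EnemyHitCheck is an animation notify state that checks for melee hits from BP_Enemy during an animation window.
; Each tick it debug-draws a Camera-channel sphere trace along the Melee component's Start socket up vector, spanning the Start-to-End distance.
; It finds the enemy with GetActorOfClass, not from the animated mesh's owner.
; Each hit actor receives negative base damage once per window, via an ignore list cleared on begin.
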(fn ReceivedNotifyTick
  (params (MeshComp :type Skeletal%20Mesh%20Component%20Object%20Reference) (Animation :type Anim%20Sequence%20Base%20Object%20Reference) (FrameDeltaTime :type Float%20%28single-precision%29))
  (bind _returnvalue (Actor|GetActorOfClass MeshComp "/Game/Blueprint/Enemy/BP_Enemy.BP_Enemy_C"))
  (bind _outhit (Collision|SphereTraceByChannel MeshComp (Transformation|GetSocketLocation (Variables|/Game/Blueprint/Enemy/BP_Enemy.BP_Enemy_C|GetMelee _returnvalue) "Start") (+ (* (Math|Vector|GetUpVector (Transformation|GetSocketRotation (Variables|/Game/Blueprint/Enemy/BP_Enemy.BP_Enemy_C|GetMelee _returnvalue) "Start")) (Math|Vector|VectorLength (- (Transformation|GetSocketLocation (Variables|/Game/Blueprint/Enemy/BP_Enemy.BP_Enemy_C|GetMelee _returnvalue) "End") (Transformation|GetSocketLocation (Variables|/Game/Blueprint/Enemy/BP_Enemy.BP_Enemy_C|GetMelee _returnvalue) "Start")))) (Transformation|GetSocketLocation (Variables|/Game/Blueprint/Enemy/BP_Enemy.BP_Enemy_C|GetMelee _returnvalue) "Start")) 1e+01 "TraceTypeQuery2" false (Variables|Default|GetIgnoreActors) "ForDuration"))
  (if (Utilities|Array|ContainsItem (Variables|Default|GetIgnoreActors) (.HitActor (Collision|BreakHitResult _outhit)))
    _
    (else
      (Utilities|Array|AddUnique (Variables|Default|GetIgnoreActors) (.HitActor (Collision|BreakHitResult _outhit)))
      (Game|Damage|ApplyDamage (.HitActor (Collision|BreakHitResult _outhit)) -1e+01 0 0)))
  (return false))

(fn ReceivedNotifyBegin
  (params (MeshComp :type Skeletal%20Mesh%20Component%20Object%20Reference) (Animation :type Anim%20Sequence%20Base%20Object%20Reference) (TotalDuration :type Float%20%28single-precision%29))
  (Utilities|Array|Clear (Variables|Default|GetIgnoreActors))
  (return false))